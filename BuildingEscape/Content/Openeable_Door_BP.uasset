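; Openable door actor that swings open and closed through the OpenDoor events OpenDoorPls and CloseDoorPls.
; It stores its starting rotation on BeginPlay, and a timeline adds an animated yaw angle to that rotation.
; Opening plays the timeline and closing reverses it, while an event track on the same timeline plays the Doorlock sound at the door's location.
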(event OpenDoorPls(OpenDoor)
  (bind _openangle (Timeline|Timeline_0 Play)
    (:Update
      (Transformation|SetActorRotation (Math|Rotator|CombineRotators (Variables|Default|GetinitialRotation) (Math|Rotator|MakeRotator 0.0 0.0 _openangle))))
    (:NewTrack_1
      (Audio|PlaySoundatLocation "/Game/Sounds/door-lock.door-lock" (Transformation|GetActorLocation) "0, 0, 0" 1.0 1.0 0.0 0 0 0))))

(event CloseDoorPls(OpenDoor)
  (bind _openangle (Timeline|Timeline_0 Reverse)
    (:Update
      (Transformation|SetActorRotation (Math|Rotator|CombineRotators (Variables|Default|GetinitialRotation) (Math|Rotator|MakeRotator 0.0 0.0 _openangle))))
    (:NewTrack_1
      (Audio|PlaySoundatLocation "/Game/Sounds/door-lock.door-lock" (Transformation|GetActorLocation) "0, 0, 0" 1.0 1.0 0.0 0 0 0))))

(event EventBeginPlay
  (Variables|Default|SetinitialRotation (Transformation|GetActorRotation)))

(fn ConstructionScript)